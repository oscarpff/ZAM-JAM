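; BP_Burbuja is an AI-driven pawn that wanders randomly and keeps a text arrow turned toward the player.
; A looping one-second timer runs its behavior check, which starts an AI move to a random reachable nearby point when not busy.
; The busy flag clears only when the move succeeds.
; Each tick, ArrowTexto yaws to face the player character, with pitch and roll held at zero.
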(event Custom|Comportamiento%20y%20Necesidades
  (if (not (Variables|Default|GetOcupado?))
    (CallFunction|Coordenadas)))

(event Custom|Coordenadas
  (Variables|Default|SetOcupado? true)
  (AI|AIMoveTo self (.RandomLocation (AI|Navigation|GetRandomReachablePointinRadius (Transformation|GetActorLocation) 1e+03 0 0)) 0 5.0 false
    (:OnSuccess
      (Variables|Default|SetOcupado? false))))

(event EventBeginPlay
  (Utilities|FlowControl|Sequence
    (:then_0
      (Utilities|Time|SetTimerbyEvent (delegate Custom|Comportamiento%20y%20Necesidades) 1.0 true))))

(event EventTick
  (params (DeltaSeconds :type Float%20%28single-precision%29))
  (Utilities|FlowControl|Sequence
    (:then_0
      (Transformation|SetWorldRotation (Variables|Default|GetArrowTexto) (Math|Rotator|MakeRotator 0.0 0.0 (.yaw (Math|Rotator|FindLookatRotation (Transformation|GetWorldLocation (Variables|Default|GetArrowTexto)) (Transformation|GetActorLocation (Game|GetPlayerCharacter 0))))) false false))))

(fn ConstructionScript)