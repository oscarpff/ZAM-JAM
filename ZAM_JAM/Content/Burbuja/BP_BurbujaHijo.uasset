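; BP_BurbujaHijo is a child bubble pawn that follows the first-person character using AI movement.
; It calls its parent logic, marks itself Ocupado on BeginPlay, and reissues AIMoveTo toward the player every Tick while IrAhi is false.
; The Iralli event sends it to supplied coordinates instead.
; Box overlap events are empty, and an up-down bobbing timeline is left unconnected.
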(event OnComponentBeginOverlap(Box)
  (params (OverlappedComponent :type Primitive%20Component%20Object%20Reference) (OtherActor :type Actor%20Object%20Reference) (OtherComp :type Primitive%20Component%20Object%20Reference) (OtherBodyIndex :type Integer) (bFromSweep :type Boolean) (SweepResult :type Hit%20Result%20Structure%20%28by%20ref%29)))

(event OnComponentEndOverlap(Box)
  (params (OverlappedComponent :type Primitive%20Component%20Object%20Reference) (OtherActor :type Actor%20Object%20Reference) (OtherComp :type Primitive%20Component%20Object%20Reference) (OtherBodyIndex :type Integer)))

(event Custom|Ir%20alli
  (params (Coordenadas :type Vector))
  (AI|AIMoveTo self Coordenadas 0 5.0 false))

(event EventBeginPlay
  (|CallParentFunction)
  (Variables|Default|SetOcupado? true))

(event Collision|EventActorBeginOverlap
  (params (OtherActor :type Actor%20Object%20Reference)))

(event EventTick
  (params (DeltaSeconds :type Float%20%28single-precision%29))
  (|CallParentFunction DeltaSeconds)
  (Utilities|FlowControl|Sequence
    (:then_0
      (if (not (Variables|Default|GetIr%20ahi))
        (bind _returnvalue (Actor|GetActorOfClass "/Game/FirstPerson/Blueprints/BP_FirstPersonCharacter.BP_FirstPersonCharacter_C"))
        (AI|AIMoveTo self "0, 0, 0" _returnvalue 1e+02 false)))))

(fn ConstructionScript
  (|CallParentFunction))