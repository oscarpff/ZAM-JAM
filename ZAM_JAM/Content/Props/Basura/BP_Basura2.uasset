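; BP_Basura2 is a trash prop that the player can clean up.
; On BeginPlay it binds its Limpiar event to the first-person character's dispatcher, then filters each broadcast after a short delay by checking whether the character's Itemtouching is itself.
; A one-time pass plays a sound and runs a timeline that shrinks the mesh to zero, activates Niagara and calls SumarBasura on the character once.
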(event Custom|Limpiar
  (Utilities|FlowControl|Delay 0.5)
  (if (== (Variables|/Game/FirstPerson/Blueprints/BP_FirstPersonCharacter.BP_FirstPersonCharacter_C|GetItemtouching (stale EventBeginPlay _asbp_first_person_character)) self)
    (Utilities|FlowControl|DoOnce false
      (:Completed
        (Audio|SpawnSound2D "/Game/Audios/AudioBasura.AudioBasura" 1.0 1.0 0.0 0)
        (bind _escala (Timeline|Scale Play)
          (:Update
            (Transformation|SetRelativeScale3D (Variables|Default|GetBasura) (Math|Vector|Lerp(Vector) "0.300000,0.300000,0.300000" "0, 0, 0" _escala))
            (Components|Activation|Activate (Variables|Default|GetNiagara) false)
            (Utilities|FlowControl|DoOnce false
              (:Completed
                (Default|SumarBasura (Variables|Default|GetAs%20BP%20First%20Person%20Character))))))))))

(event EventBeginPlay
  (bind _asbp_first_person_character (Utilities|Casting|CastToBP_FirstPersonCharacter (Game|GetPlayerCharacter 0)))
  (bind _output_get (Variables|Default|SetAs%20BP%20First%20Person%20Character _asbp_first_person_character))
  (EventDispatchers|BindEventtoLimpiar _output_get (delegate Custom|Limpiar)))

(event EventTick
  (params (DeltaSeconds :type Float%20%28single-precision%29)))

(fn ConstructionScript)