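; Cleanable trash decal prop that the player removes with the first-person character's clean (Limpiar) action.
; On BeginPlay it binds to the character's Limpiar event, then after a half-second delay checks whether it is the character's touched item.
; If so, a one-shot timeline shrinks its plane to zero, and the first update calls SumarBasura once to add to the trash count.
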(event Custom|Limpiar
  (Utilities|FlowControl|Delay 0.5)
  (if (== (Variables|/Game/FirstPerson/Blueprints/BP_FirstPersonCharacter.BP_FirstPersonCharacter_C|GetItemtouching (stale EventBeginPlay _asbp_first_person_character)) self)
    (Utilities|FlowControl|DoOnce false
      (:Completed
        (bind _escala (Timeline|Timeline Play)
          (:Update
            (Transformation|SetRelativeScale3D (Variables|Default|GetPlane) (Math|Vector|Lerp(Vector) "1.000000,1.000000,1.000000" "0, 0, 0" _escala))
            (Utilities|FlowControl|DoOnce false
              (:Completed
                (Default|SumarBasura (Variables|Default|GetAs%20BP%20First%20Person%20Character))))))))))

(event EventBeginPlay
  (bind _asbp_first_person_character (Utilities|Casting|CastToBP_FirstPersonCharacter (Game|GetPlayerCharacter 0)))
  (bind _output_get (Variables|Default|SetAs%20BP%20First%20Person%20Character _asbp_first_person_character))
  (EventDispatchers|BindEventtoLimpiar _output_get (delegate Custom|Limpiar)))

(event Collision|EventActorBeginOverlap
  (params (OtherActor :type Actor%20Object%20Reference)))

(event EventTick
  (params (DeltaSeconds :type Float%20%28single-precision%29)))

(fn ConstructionScript)