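; Light switch prop that lets the player turn a referenced point light on and off.
; On BeginPlay it binds to the first-person character's Encender dispatcher, and reacts only when it is that character's Itemtouching item, otherwise printing a debug string.
; A FlipFlop alternates between tilting the switch with the light visible and resetting it with the light hidden, starting with on.
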(event Custom|Encender/Apagar
  (bind _interruptor_interruptor (Variables|Default|GetInterruptor_Interruptor))
  (bind _luz (Variables|Default|GetLuz))
  (bind _pointlightcomponent (Variables|/Script/Engine.PointLight|GetPointLightComponent _luz))
  ;[1 1 1] Encender / Apagar luces
  (Utilities|FlowControl|FlipFlop
    (:A
      (Transformation|SetRelativeRotation _interruptor_interruptor "-17.000000,0.000000,0.000000" false false)
      (Rendering|SetVisibility _pointlightcomponent true false))
    (:B
      (Transformation|SetRelativeRotation _interruptor_interruptor "0, 0, 0" false false)
      (Rendering|SetVisibility _pointlightcomponent false false))))

(event Custom|Switch
  ;[1 1 1] Bind Evento al Player
  (if (== (Variables|/Game/FirstPerson/Blueprints/BP_FirstPersonCharacter.BP_FirstPersonCharacter_C|GetItemtouching (stale EventBeginPlay _asbp_first_person_character)) self)
    (CallFunction|Encender/Apagar)
    (else
      (Development|PrintString "asdadsad"))))

(event EventBeginPlay
  ;[1 1 1] Bind Evento al Player
  (bind _asbp_first_person_character (Utilities|Casting|CastToBP_FirstPersonCharacter (Game|GetPlayerCharacter 0)))
  (bind _output_get (Variables|Default|SetAs%20BP%20First%20Person%20Character _asbp_first_person_character))
  (EventDispatchers|BindEventtoEncender _output_get (delegate Custom|Switch)))

(fn ConstructionScript)